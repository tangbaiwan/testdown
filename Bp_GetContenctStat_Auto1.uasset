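; Actor Blueprint that checks whether a socket connection to a given IP and port can be opened through a referenced DSActor.
; GetCurrentStat creates the socket, requests the spend list with Body on success, then closes the socket and returns the connection result.
; An invalid DSActor only prints a placeholder message.
; The event graph is inactive, holding just an unwired CreateSocket call with a hardcoded address.
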(event EventBeginPlay)

(event Collision|EventActorBeginOverlap
  (params (OtherActor :type Actor%20Object%20Reference)))

(event EventTick
  (params (DeltaSeconds :type Float%20%28single-precision%29)))

(fn ConstructionScript)

(fn GetCurrentStat
  (params (IpString :type String) (PortNumer :type Integer))
  (bind _dsactor (Variables|Default|GetDSActor))
  (Utilities|IsValid _dsactor
    (:Is%20Valid
      (bind _returnvalue (Class|DSActorComponent|CreateSocket _dsactor IpString PortNumer))
      (LocalVariables|SetCurrenttat _returnvalue)
      (if (LocalVariables|GetCurrenttat)
        (Class|DSActorComponent|GetSpendList (Variables|Default|GetDSActor) (Variables|Default|GetBody)))
      (Class|DSActorComponent|CloseSocket _dsactor)
      (return (LocalVariables|GetCurrenttat)))
    (:Is%20Not%20Valid
      (Development|PrintString "Hello"))))