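; Startup actor for a "DST" tool that opens the main UMG widget in its own titled window and manages the displayed human character.
; On BeginPlay it registers itself and the DirectionalLight with the DSINI game instance, spawns the human and creates a CineCamera as view target.
; SpawnHuman replaces the current actor with the selected HumanList class, preserving its location and rotation through DSINI.
; The C key alternates between possessing the DefaultPawn and blending to the camera.
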(event EventBeginPlay
  (Utilities|FlowControl|Sequence
    (:then_0
      (Development|ExecuteConsoleCommand "r.Streaming.PoolSize 0" 0))
    (:then_1
      (bind _asdsini (Utilities|Casting|CastToDSINI (Game|GetGameInstance)))
      (Variables|Default|SetDSINI _asdsini)
      (Variables|/DSHumanComponent/DSINI.DSINI_C|SetConsoleBp _asdsini self))
    (:then_2
      (bind _returnvalue (UserInterface|CreateWidget "/Game/UMG/UMG_Main.UMG_Main_C"))
      (Variables|/Game/UMG/UMG_Main.UMG_Main_C|SetDSWindows _returnvalue self)
      (CallFunction|SpawnHuman)
      (bind _returnvalue_2 (Actor|GetActorOfClass "/Script/Engine.DirectionalLight"))
      (Variables|/DSHumanComponent/DSINI.DSINI_C|SetSun (Variables|Default|GetDSINI) _returnvalue_2)
      (bind _returnvalue_3 (Class|GameUserSettings|GetDefaultWindowPosition))
      (Class|DSWindows|CreateWindow _returnvalue true "DST" (Math|Conversions|ToVector2D(IntPoint) _returnvalue_3) "(X=1080.000000,Y=720.000000)" true true true true))
    (:then_3
      (bind _returnvalue_4 (Game|SpawnActorfromClass "/Script/CinematicCamera.CineCameraActor" (Math|Transform|MakeTransform "0, 0, 0" "0, 0, 0" "1.000000,1.000000,1.000000") "Undefined" 0 0))
      (Variables|Default|SetCamera _returnvalue_4)
      (Game|Player|SetViewTargetwithBlend (Game|GetPlayerController 0) (Variables|Default|GetCamera) 0.0 "VTBlend_EaseIn" 0.0 false)
      (bind _returnvalue_5 (Actor|GetActorOfClass "/Script/Engine.DefaultPawn"))
      (Variables|Default|SetPawn _returnvalue_5))
    (:then_4
      (Utilities|FlowControl|Delay 0.2)
      (Utilities|IsValid (Variables|Default|GetActor)))))

(event Input|KeyboardEvents|C
  (params (Key :type Key%20Structure :default "None"))
  (bind _returnvalue (Game|GetPlayerController 0))
  (:Pressed
    (Utilities|FlowControl|FlipFlop
      (:A
        (Pawn|Possess _returnvalue (Variables|Default|GetPawn)))
      (:B
        (Game|Player|SetViewTargetwithBlend _returnvalue (Variables|Default|GetCamera) 0.0 "VTBlend_EaseIn" 0.0 false)))))

(fn ConstructionScript)

(fn ClearHuman
  (bind _dsini (Variables|Default|GetDSINI))
  (bind _dsini_2 (Variables|Default|GetDSINI))
  (bind _actor (Variables|/DSHumanComponent/DSINI.DSINI_C|GetActor _dsini))
  (Utilities|IsValid _actor
    (:Is%20Valid
      (Variables|/DSHumanComponent/DSINI.DSINI_C|SetHumanLoc _dsini_2 (Transformation|GetActorLocation _actor))
      (Variables|/DSHumanComponent/DSINI.DSINI_C|SetHumanRot _dsini_2 (Transformation|GetActorRotation _actor))
      (Actor|DestroyActor _actor))))

(fn SpawnHuman
  (bind _dsini (Variables|Default|GetDSINI))
  (CallFunction|ClearHuman)
  (bind _returnvalue (Game|SpawnActorfromClass (Utilities|ResolveSoftReference (.class (Utilities|Array|Get(acopy) (Variables|/DSHumanComponent/DSINI.DSINI_C|GetHumanList _dsini) (Variables|/DSHumanComponent/DSINI.DSINI_C|GetSelectedHuman _dsini)))) (Math|Transform|MakeTransform (Variables|/DSHumanComponent/DSINI.DSINI_C|GetHumanLoc _dsini) (Variables|/DSHumanComponent/DSINI.DSINI_C|GetHumanRot _dsini) "1.000000,1.000000,1.000000") "Undefined" 0 0))
  (Variables|/DSHumanComponent/DSINI.DSINI_C|SetActor (Variables|Default|GetDSINI) _returnvalue)
  (Variables|Default|SetActor _returnvalue))